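; BP_Enemy is an enemy combatant Blueprint in a turn-based combat test.
; Its DealDamage event subtracts the given damage from Health, with no death check.
; StartTurn prints a turn message, waits briefly, then finds the TurnBasedBattleMode actor and calls ChangeTurn to hand the turn back, without taking any action.
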(event `DealDamage`
  (params (Damage :type "Float (double-precision)"))
  ;[1 1 1] Simple deal damage event
  (set `self.Health` (- (`self.Health`) Damage)))

(event `Start Turn`
  (`KismetSystemLibrary.PrintString` "Enemy turn")
  (`KismetSystemLibrary.Delay` 1.0)
  (bind _returnvalue (`GameplayStatics.GetActorOfClass` "/Game/TurnBasedCombatTest/TurnBasedBattleMode.TurnBasedBattleMode_C"))
  (`/Game/TurnBasedCombatTest/TurnBasedBattleMode.Change Turn` _returnvalue))

(fn `UserConstructionScript`
  (`parent.UserConstructionScript`))