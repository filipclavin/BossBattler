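; BP_AttackAbility is an attack ability in a turn-based skill system that changes an enemy's health.
; On BeginPlay it caches the BP_TurnBasedCharacter as Target and an Enemy, each found by class lookup.
; The AB_FireAttack event runs AttackFunction, which writes the result of AttackSkill directly into the enemy's Health.
; A separate Attack function calls ManaCost on the character and is not called within this graph.
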(event `self.ReceiveBeginPlay`
  (bind _returnvalue (`GameplayStatics.GetActorOfClass` "/Game/Blueprints/Character/BP_TurnBasedCharacter.BP_TurnBasedCharacter_C"))
  (set `self.Target` _returnvalue)
  (bind _returnvalue_2 (`GameplayStatics.GetActorOfClass` "/Game/TurnBasedCombatTest/Enemy.Enemy_C"))
  (set `self.Enemy` _returnvalue_2))

(event `AB_FireAttack`
  (`self.AttackFunction`))

(fn `Attack`
  (`/Game/Blueprints/Character/BP_TurnBasedCharacter.ManaCost` (`self.Target`)))

(fn `AttackFunction`
  (bind _enemyhealth (`self.AttackSkill` (`self.Skill`)))
  (set `/Game/TurnBasedCombatTest/Enemy.Health` _enemyhealth (`self.Enemy`)))