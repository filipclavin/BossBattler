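; BP_Skill is a skill Blueprint for a turn-based combat system, holding references to the player character and an enemy.
; On BeginPlay it finds and stores the first BP_TurnBasedCharacter and BP_Enemy actors in the level.
; Cast subtracts ManaCost from the character's Mana, clamped between zero and MaxMana, and prints the new value; the stored enemy reference is not used here.
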(event `self.ReceiveBeginPlay`
  (`|ExecutionSequence`
    (:`then_0`
      (bind _returnvalue (`GameplayStatics.GetActorOfClass` "/Game/Blueprints/Character/BP_TurnBasedCharacter.BP_TurnBasedCharacter_C"))
      (set `self.Character` _returnvalue))
    (:`then_1`
      (bind _returnvalue_2 (`GameplayStatics.GetActorOfClass` "/Game/TurnBasedCombatTest/BP_Enemy.BP_Enemy_C"))
      (set `self.Enemy` _returnvalue_2))))

(fn `Cast`
  (bind _output_get (set `TurnedBasedCharacter.Mana` (`KismetMathLibrary.FClamp` (- (`TurnedBasedCharacter.Mana` (`self.Character`)) (`self.ManaCost`)) 0.0 (`TurnedBasedCharacter.MaxMana` (`self.Character`))) (`self.Character`)))
  (`KismetSystemLibrary.PrintString` (`KismetStringLibrary.Conv_DoubleToString` _output_get)))