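; Turn-based character Blueprint that tracks Mana and Heat resources and casts fireball and ice beam spells.
; Small functions pass each resource through clamp-style add or reduce helpers and store the result; mana cost reuses the ManaRegen amount.
; Number keys 1–4 trigger these functions, apparently for testing.
; Fire and IceAttack events call Cast on their spell references without touching resources, while FireAttack is an empty stub.
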(event `self.ReceiveBeginPlay`)

(event `self.ReceiveTick`
  (params (DeltaSeconds :type "Float (single-precision)")))

(event `Key|One`
  (params (Key :type "Key Structure"))
  ;[1 1 1] TEst
  (:`Pressed`
    (`self.Mana Regen`)))

(event `FireAttack`)

(event `Key|Two`
  (params (Key :type "Key Structure"))
  ;[1 1 1] TEst
  (:`Pressed`
    (`self.ManaCost`)))

(event `Key|Three`
  (params (Key :type "Key Structure"))
  ;[1 1 1] TEst
  (:`Pressed`
    (`self.HeatCost`)))

(event `Key|Four`
  (params (Key :type "Key Structure"))
  ;[1 1 1] TEst
  (:`Pressed`
    (`self.IncreaseHeat`)))

(event `IceAttack`
  (`/Game/Blueprints/SkillSystem/BP_Skill.Cast` (`self.BP_IceBeam`)))

(event `Fire`
  (`/Game/Blueprints/SkillSystem/BP_Skill.Cast` (`self.BP_FireBall`)))

(fn `HeatCost`
  (bind _returnvalue (`self.RemoveHeat` (`self.Heat`) (`self.HCost`)))
  (set `self.Heat` _returnvalue))

(fn `IncreaseHeat`
  (bind _returnvalue (`self.AddHeat` (`self.Heat`) (`self.HeatRegen`) (`self.MaxHeat`)))
  (set `self.Heat` _returnvalue))

(fn `Mana Regen`
  (bind _returnvalue (`self.RegenMana` (`self.Mana`) (`self.ManaRegen`) (`self.MaxMana`)))
  (set `self.Mana` _returnvalue))

(fn `ManaCost`
  (bind _returnvalue (`self.ReduceMana` (`self.Mana`) (`self.ManaRegen`)))
  (set `self.Mana` _returnvalue))

(fn `UserConstructionScript`)